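; BP_Eagle is a moving hazard that flies along the world Y axis and ends the game when it overlaps a chicken.
; Each tick it moves with a swept world offset scaled by Speed, counts down Lifetime to destroy itself, and plays the Eagle sound once after a short delay.
; On overlap with BP_Chicken it hides the chicken's mesh and calls that chicken's SetGameOverForGameMode.
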(event EventBeginPlay)

(event EventTick
  (params (DeltaSeconds :type Float%20%28single-precision%29))
  (Transformation|AddActorWorldOffset (Math|Vector|MakeVector 0.0 (* DeltaSeconds (Variables|Default|Getspeed)) 0.0) true)
  (if (>= (Variables|Default|Getlifetime) 0.0)
    (Variables|Default|Setlifetime (- (Variables|Default|Getlifetime) DeltaSeconds))
    (else
      (Actor|DestroyActor)))
  (if (not (Variables|Default|GetplayingEagleSound))
    (bind _output_get (Variables|Default|SetsoundOffset (+ (Variables|Default|GetsoundOffset) DeltaSeconds)))
    (if (>= _output_get 0.5)
      (Variables|Default|SetplayingEagleSound true)
      (Audio|PlaySound2D "/Game/Media/Sounds/eagle.eagle" 1.0 1.0 0.0 0 0))))

(event Collision|EventActorBeginOverlap
  (params (OtherActor :type Actor%20Object%20Reference))
  (bind _asbp_chicken (Utilities|Casting|CastToBP_Chicken OtherActor))
  (Rendering|SetVisibility (Variables|/Game/Blueprints/BP_Chicken.BP_Chicken_C|GetStaticMesh _asbp_chicken) false false)
  (Default|SetGameOverforGameMode _asbp_chicken))

(fn ConstructionScript)