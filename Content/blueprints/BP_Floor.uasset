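; BP_Floor is a floor actor that shows a grass, road or water mesh according to its FloorType.
; On BeginPlay, a MultiGate uses FloorType as its start index to route to SetMesh with the matching mesh.
; SetMesh applies it and creates a dynamic instance of a shared color material.
; Non-traversable floors are darkened by lowering that instance's "darkness" vector parameter.
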(event EventBeginPlay
  (Utilities|FlowControl|MultiGate false false (Variables|Default|GetfloorType)
    (:Out%200
      (CallFunction|SetMesh "/Game/media/meshes/grass.grass"))
    (:Out%201
      (CallFunction|SetMesh "/Game/media/meshes/road.road"))
    (:Out%202
      (CallFunction|SetMesh "/Game/media/meshes/water.water"))))

(event Collision|EventActorBeginOverlap
  (params (OtherActor :type Actor%20Object%20Reference)))

(event EventTick
  (params (DeltaSeconds :type Float%20%28single-precision%29)))

(fn ConstructionScript)

(fn SetMesh
  (params (staticMesh :type Static%20Mesh%20Object%20Reference))
  (Components|StaticMesh|SetStaticMesh (Variables|Default|GetFloorMesh) staticMesh)
  (bind _returnvalue (Rendering|Material|CreateDynamicMaterialInstance (Variables|Default|GetFloorMesh) 0 "/Game/media/meshes/M_chicken__colors_png.M_chicken__colors_png" "None" :!class /Script/Engine.PrimitiveComponent))
  (bind _output_get (Variables|Default|SetmaterialInstance _returnvalue))
  (if (not (Variables|Default|Gettraversable))
    (CallFunction|DarkenMesh _output_get)))

(fn DarkenMesh
  (params (materialInstance :type Material%20Instance%20Dynamic%20Object%20Reference))
  (bind _returnvalue (Rendering|Material|GetVectorParameterValue materialInstance "darkness" :!class /Script/Engine.MaterialInstanceDynamic))
  (Rendering|Material|SetVectorParameterValue materialInstance "darkness" (Math|Conversions|ToLinearColor(Float) (- (.R (Utilities|Struct|BreakLinearColor _returnvalue)) 0.4)) :!class /Script/Engine.MaterialInstanceDynamic))