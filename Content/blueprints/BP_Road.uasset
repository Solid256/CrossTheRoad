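; BP_Road is a road chunk that gives the chicken a lane of vehicle traffic to cross.
; On BeginPlay it spawns left, center and right floor pieces, with only the center marked traversable, plus optional line props.
; It then adds a vehicle spawner on a random side, passing it the facing and chicken reference, and builds a row of landing nodes.
; Destroying the road also destroys its vehicle spawners.
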(event EventBeginPlay
  (bind _self self)
  (bind _props (Variables|Default|Getprops))
  (bind _list (Utilities|Struct|BreakArrayOfActor _props))
  (bind (_transformmid _transformleft _transformright _ypos) (CallFunction|CalcFloorTransform))
  (bind _returnvalue (Game|SpawnActorfromClass "/Game/blueprints/BP_Floor.BP_Floor_C" _transformleft "Undefined" 0 1 false _self 0))
  (Variables|Default|SetleftFloor _returnvalue)
  (bind _returnvalue_2 (Game|SpawnActorfromClass "/Game/blueprints/BP_Floor.BP_Floor_C" _transformmid "Undefined" 0 1 true _self 0))
  (Variables|Default|SetcenterFloor _returnvalue_2)
  (bind _returnvalue_3 (Game|SpawnActorfromClass "/Game/blueprints/BP_Floor.BP_Floor_C" _transformright "Undefined" 0 1 false _self 0))
  (Variables|Default|SetrightFloor _returnvalue_3)
  (if (Variables|Default|GethasLines)
    (bind _returnvalue_4 (Game|SpawnActorfromClass "/Game/blueprints/BP_Road_Lines.BP_Road_Lines_C" (Math|Transform|MakeTransform (Math|Vector|MakeVector -2e+03 (- _ypos -1e+02) 0.0)) "Undefined" 0 true 0))
    (Utilities|Array|Add _list _returnvalue_4)
    (bind _returnvalue_5 (Game|SpawnActorfromClass "/Game/blueprints/BP_Road_Lines.BP_Road_Lines_C" (Math|Transform|MakeTransform (Math|Vector|MakeVector 0.0 (- _ypos -1e+02) 0.0)) "Undefined" 0 false 0))
    (Utilities|Array|Add _list _returnvalue_5)
    (bind _returnvalue_6 (Game|SpawnActorfromClass "/Game/blueprints/BP_Road_Lines.BP_Road_Lines_C" (Math|Transform|MakeTransform (Math|Vector|MakeVector 2e+03 (- _ypos -1e+02) 0.0)) "Undefined" 0 true 0))
    (Utilities|Array|Add _list _returnvalue_6))
  (CallFunction|ConstructVehicleSpawner _ypos)
  (CallFunction|ConstructLandingNodes))

(event Collision|EventActorBeginOverlap
  (params (OtherActor :type Actor%20Object%20Reference)))

(event EventTick
  (params (DeltaSeconds :type Float%20%28single-precision%29)))

(event EventDestroyed
  (for _array_element (.list (Variables|Default|GetvehicleSpawners))
    (Actor|DestroyActor _array_element)))

(fn ConstructionScript)

(fn ConstructVehicleSpawner
  (params (posY :type Float%20%28single-precision%29))
  (bind _output_get (LocalVariables|SetfacingLeft (Math|Random|RandomBool)))
  (if _output_get
    (LocalVariables|SetposX 2.8e+03)
    (else
      (bind _output_get_2 (LocalVariables|SetposX -2.8e+03))))
  (bind _returnvalue (Game|SpawnActorfromClass "/Game/blueprints/BP_Vehicle_Spawner.BP_Vehicle_Spawner_C" (Math|Transform|MakeTransform (Math|Vector|MakeVector _output_get_2 posY -1e+01)) "Undefined" 0 _output_get (Variables|Default|GetchickenRef) 0))
  (Utilities|Array|Add (.list (Variables|Default|GetvehicleSpawners)) _returnvalue))

(fn ConstructLandingNodes
  (Variables|Default|SetcurZPositionForLandingNode -3e+01)
  (for _index (range 0 8)
    (CallFunction|ConstructLandingNode false)))