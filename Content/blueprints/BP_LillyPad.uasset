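; Lily pad platform that the chicken can land on, with a chance to carry a coin.
; On BeginPlay it picks a random yaw spin rate and, one time in three, spawns a BP_Coin at its location.
; Each tick it plays a sound as a jump onto it starts, runs the bouncing animation, and keeps spinning unless a chicken is on top.
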(event EventBeginPlay
  (|CallParentFunction)
  (Variables|Default|Setrotation (Math|Rotator|MakeRotator 0.0 0.0 (Math|Random|RandomFloatinRange -2e+01 2e+01)))
  (switch int (Math|Random|RandomInteger 3)
    (:0
      (Game|SpawnActorfromClass "/Game/Blueprints/BP_Coin.BP_Coin_C" (Math|Transform|MakeTransform (Transformation|GetActorLocation)) "Undefined" 0 0))))

(event Collision|EventActorBeginOverlap
  (params (OtherActor :type Actor%20Object%20Reference)))

(event EventTick
  (params (DeltaSeconds :type Float%20%28single-precision%29))
  (CallFunction|AttemptPlayJumpedonSound)
  (CallFunction|BouncingAnimation DeltaSeconds)
  (if (not (Variables|Default|GethasChickenOnTopOf))
    (Transformation|AddActorLocalRotation (* (Variables|Default|Getrotation) DeltaSeconds) false false)))

(fn ConstructionScript)

(fn AttemptPlayJumpedonSound
  (if (and (== (Variables|Default|GetcurJumpedOnTime) 0.0) (Variables|Default|GetisBeingJumpedOn))
    (Audio|PlaySound2D "/Game/Media/Sounds/lily_pad.lily_pad" 1.0 1.0 0.0 0 0)))