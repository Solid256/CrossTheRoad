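; Main game camera that auto-scrolls along a track while easing toward chicken-driven X and Y offsets.
; BeginPlay derives its base position from CameraDistance.
; Tick accumulates forward travel on Y when tracking is enabled and advances separate ease-out blends for each offset axis.
; It then sums base, tracking, eased and log X offsets into the actor location; a helper function zeroes the log offset.
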(event EventBeginPlay
  (bind _cameradistance (Variables|Default|GetcameraDistance))
  (Variables|Default|SetdefaultXPos (+ (* _cameradistance 0.335) -2e+02))
  (Variables|Default|SetdefaultYPos (+ (* _cameradistance 0.84) -6e+02))
  (Variables|Default|SetdefaultZPos (* _cameradistance 1.0)))

(event Collision|EventActorBeginOverlap
  (params (OtherActor :type Actor%20Object%20Reference)))

(event EventTick
  (params (DeltaSeconds :type Float%20%28single-precision%29))
  (if (Variables|Default|GettrackingForwards)
    (CallFunction|CalcTrackPosition DeltaSeconds))
  (if (< (Variables|Default|GetinterpAlphaX) 1.0)
    (CallFunction|CalcInterpOffsetX DeltaSeconds))
  (if (< (Variables|Default|GetinterpAlphaY) 1.0)
    (CallFunction|CalcInterpOffsetY DeltaSeconds))
  (CallFunction|CalcFinalPosition))

(fn ConstructionScript)

(fn CalcFinalPosition
  (bind _autotrackvelocity (Variables|Default|GetautoTrackVelocity))
  (Transformation|SetActorLocation (Math|Vector|MakeVector (+ (Variables|Default|GetdefaultXPos) (.x _autotrackvelocity) (Variables|Default|GetinterpOffsetResultX) (Variables|Default|GetlogOffsetX)) (+ (Variables|Default|GetdefaultYPos) (.y _autotrackvelocity) (Variables|Default|GetinterpOffsetResultY) (Variables|Default|GettotalTrackDistanceY)) (+ (Variables|Default|GetdefaultZPos) (.z _autotrackvelocity))) false false))

(fn CalcInterpOffsetX
  (params (deltaTime :type Float%20%28single-precision%29))
  (bind _output_get (Variables|Default|SetinterpAlphaX (+ deltaTime (Variables|Default|GetinterpAlphaX))))
  (Variables|Default|SetinterpOffsetResultX (Math|Interpolation|Ease "EaseOut" _output_get (Variables|Default|GetstartChickenInterpPosX) (Variables|Default|GetchickenInterpOffsetX) 2.0)))

(fn CenterInterpOffsetwithLogXPos
  (Variables|Default|SetlogOffsetX 0.0))

(fn CalcTrackPosition
  (params (deltaTime :type Float%20%28single-precision%29))
  (bind _output_get (Variables|Default|SetautoTrackVelocity (* (Variables|Default|GetcameraDir) (* deltaTime (Variables|Default|GetcameraSpeed)))))
  (Variables|Default|SettotalTrackDistanceY (+ (.y _output_get) (Variables|Default|GettotalTrackDistanceY))))

(fn CalcInterpOffsetY
  (params (deltaTime :type Float%20%28single-precision%29))
  (bind _output_get (Variables|Default|SetinterpAlphaY (+ deltaTime (Variables|Default|GetinterpAlphaY))))
  (Variables|Default|SetinterpOffsetResultY (Math|Interpolation|Ease "EaseOut" _output_get (Variables|Default|GetstartChickenInterpPosY) (Variables|Default|GetchickenInterpOffsetY) 2.0)))