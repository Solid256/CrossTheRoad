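; Bush actor that randomizes its look in the Construction Script, adding variety to placed foliage.
; A random roll sets one of three quarter-turn rotations, then a second roll picks one of three tree static meshes.
; A zero on the first roll skips both steps, and a three on the second leaves the mesh unchanged.
; Results re-roll whenever construction reruns; BeginPlay only calls its parent.
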(event EventBeginPlay
  (|CallParentFunction))

(event Collision|EventActorBeginOverlap
  (params (OtherActor :type Actor%20Object%20Reference)))

(event EventTick
  (params (DeltaSeconds :type Float%20%28single-precision%29)))

(fn ConstructionScript
  (bind _staticmesh (Variables|Default|GetStaticMesh))
  (switch int (Math|Random|RandomIntegerinRange 0 3)
    (:1
      (Transformation|SetActorRotation "0,90.000000, 0"))
    (:2
      (Transformation|SetActorRotation "0,180.000000, 0"))
    (:3
      (Transformation|SetActorRotation "0,270.000000, 0")))
  (switch int (Math|Random|RandomIntegerinRange 0 3)
    (:0
      (Components|StaticMesh|SetStaticMesh _staticmesh "/Game/Media/Models/Meshes/SM_Tree1.SM_Tree1"))
    (:1
      (Components|StaticMesh|SetStaticMesh _staticmesh "/Game/Media/Models/Meshes/SM_Tree2.SM_Tree2"))
    (:2
      (Components|StaticMesh|SetStaticMesh _staticmesh "/Game/Media/Models/Meshes/SM_Tree3.SM_Tree3"))))