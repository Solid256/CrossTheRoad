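; BP_Bounce is an actor that dips vertically in response to being jumped on.
; Every tick it sets its height to CachedZPosition plus an offset, advancing the animation while IsBeingJumpedOn is true.
; After a start delay, a squared-time parabola drives the offset until the timer passes its maximum and resets.
; The file never sets the jumped-on flag to true or assigns the cached height.
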(event EventBeginPlay
  (Variables|Default|SetmaxJumpedOnTime (+ (Variables|Default|GetmaxStartJumpTime) 0.2)))

(event Collision|EventActorBeginOverlap
  (params (OtherActor :type Actor%20Object%20Reference)))

(event EventTick
  (params (DeltaSeconds :type Float%20%28single-precision%29))
  (CallFunction|BouncingAnimation DeltaSeconds))

(fn ConstructionScript)

(fn JumpedonAnimation
  (params (deltaTime :type Float%20%28single-precision%29))
  (bind _output_get (Variables|Default|SetcurJumpedOnTime (+ deltaTime (Variables|Default|GetcurJumpedOnTime))))
  (if (>= (Variables|Default|GetcurJumpedOnTime) (Variables|Default|GetmaxStartJumpTime))
    (if (>= _output_get (Variables|Default|GetmaxJumpedOnTime))
      (CallFunction|ResetAnimation)
      (else
        (Variables|Default|SetjumpedOnZOffset (* (- (Math|Float|Square (- (* (- (Variables|Default|GetcurJumpedOnTime) 0.1) 8.0) 1.0)) 1.0) 2e+01))))))

(fn BouncingAnimation
  (params (InputPin :type Float%20%28single-precision%29))
  (bind _returnvalue (Transformation|GetActorLocation))
  (if (Variables|Default|GetisBeingJumpedOn)
    (CallFunction|JumpedonAnimation InputPin))
  (Transformation|SetActorLocation (Math|Vector|MakeVector (.x _returnvalue) (.y _returnvalue) (+ (Variables|Default|GetcachedZPosition) (Variables|Default|GetjumpedOnZOffset))) false false))

(fn ResetAnimation
  (Variables|Default|SetisBeingJumpedOn false)
  (Variables|Default|SetjumpedOnZOffset 0.0)
  (Variables|Default|SetcurJumpedOnTime 0.0))