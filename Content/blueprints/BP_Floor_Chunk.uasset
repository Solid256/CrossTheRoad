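; BP_Floor_Chunk is one row of floor in a chicken hopping game, with left, center and right meshes, landing nodes and props.
; Helpers compute the three floor transforms, spawn evenly spaced landing nodes along X flagged as water or not, and randomly place coins.
; Each tick it compares its Y to the chicken's, and once far enough behind destroys its floors, nodes, props and itself, leaving coins untouched.
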(event EventBeginPlay)

(event Collision|EventActorBeginOverlap
  (params (OtherActor :type Actor%20Object%20Reference)))

(event EventTick
  (params (DeltaSeconds :type Float%20%28single-precision%29))
  (CallFunction|CheckifDestroyingFloorChunk))

(fn ConstructionScript)

(fn CalcFloorTransform
  (bind _positiony (Variables|Default|GetpositionY))
  (return (Math|Transform|MakeTransform (Math|Vector|MakeVector 0.0 _positiony 0.0)) (Math|Transform|MakeTransform (Math|Vector|MakeVector -1.8e+03 _positiony 0.0)) (Math|Transform|MakeTransform (Math|Vector|MakeVector 1.8e+03 _positiony 0.0)) _positiony))

(fn DestroyMeshesLandingNodesandProps
  (for _array_element (Utilities|Struct|BreakArrayOfActor (Variables|Default|GetlandingNodes))
    (Actor|DestroyActor _array_element))
  (Actor|DestroyActor (Variables|Default|GetleftFloor))
  (Actor|DestroyActor (Variables|Default|GetrightFloor))
  (Actor|DestroyActor (Variables|Default|GetcenterFloor))
  (for _array_element_2 (Utilities|Struct|BreakArrayOfActor (Variables|Default|Getprops))
    (Actor|DestroyActor _array_element_2)))

(fn CheckifDestroyingFloorChunk
  (bind _chickenref (Variables|Default|GetchickenRef))
  (if (Utilities|IsValid _chickenref)
    (if (>= (.y (Transformation|GetActorLocation)) (+ (.y (Transformation|GetActorLocation _chickenref)) (Variables|Default|GetmaxDistBackwardsFromChicken)))
      (CallFunction|DestroyMeshesLandingNodesandProps)
      (Actor|DestroyActor))))

(fn ConstructLandingNode
  (params (isWater :type Boolean))
  (bind _returnvalue (Game|SpawnActorfromClass "/Game/blueprints/BP_LandingNode.BP_LandingNode_C" (Math|Transform|MakeTransform (Math|Vector|MakeVector (Variables|Default|GetcurXPositionForLandingNode) (.y (Transformation|GetActorLocation)) (Variables|Default|GetcurZPositionForLandingNode))) "Undefined" 0 isWater 0))
  (Variables|Default|SetcurXPositionForLandingNode (+ 2e+02 (Variables|Default|GetcurXPositionForLandingNode)))
  (Utilities|Array|Add (Utilities|Struct|BreakArrayOfActor (Variables|Default|GetlandingNodes)) _returnvalue))

(fn CreateCoinAttempt
  (if (== (Math|Random|RandomInteger 9) 0)
    (Game|SpawnActorfromClass "/Game/blueprints/BP_Coin.BP_Coin_C" (Math|Transform|MakeTransform (Math|Vector|MakeVector (Variables|Default|GetcurXPositionForLandingNode) (.y (Transformation|GetActorLocation)) (Variables|Default|GetcurZPositionForLandingNode))) "Undefined" 0 0)))