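; BP_Prop is a static mesh prop Blueprint that can optionally appear darkened.
; On BeginPlay it creates and stores a dynamic instance of the chicken colors material on the mesh's first slot.
; If the Dark flag is set, it calls Darken, which lowers the material's "darkness" vector parameter by a fixed step computed from its red channel.
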(event EventBeginPlay
  (bind _returnvalue (Rendering|Material|CreateDynamicMaterialInstance (Variables|Default|GetStaticMesh) 0 "/Game/media/meshes/M_chicken__colors_png.M_chicken__colors_png" "None" :!class /Script/Engine.PrimitiveComponent))
  (Variables|Default|SetmaterialInstance _returnvalue)
  (if (Variables|Default|Getdark)
    (CallFunction|Darken)))

(event Collision|EventActorBeginOverlap
  (params (OtherActor :type Actor%20Object%20Reference)))

(event EventTick
  (params (DeltaSeconds :type Float%20%28single-precision%29)))

(fn ConstructionScript)

(fn Darken
  (bind _materialinstance (Variables|Default|GetmaterialInstance))
  (bind _returnvalue (Rendering|Material|GetVectorParameterValue _materialinstance "darkness" :!class /Script/Engine.MaterialInstanceDynamic))
  (Rendering|Material|SetVectorParameterValue _materialinstance "darkness" (Math|Conversions|ToLinearColor(Float) (- (.R (Utilities|Struct|BreakLinearColor _returnvalue)) 0.4)) :!class /Script/Engine.MaterialInstanceDynamic))