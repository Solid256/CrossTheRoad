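; Vehicle lane spawner that emits BP_Vehicle actors sharing one facing and one random speed chosen at BeginPlay.
; Tick accumulates time and spawns at the actor's transform at randomly re-rolled intervals.
; SpawnInitialVehicles spawns at a fixed, facing-dependent X offset; its random offsets never reach the transform, and its loop exits once distance is below the threshold.
; Only these initial spawns receive ChickenRef.
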(event EventBeginPlay
  (Variables|Default|Setspeed (Math|Random|RandomFloatinRange 3e+02 6e+02))
  (CallFunction|SetNewMaxTimeforSpawn)
  (CallFunction|SpawnInitialVehicles))

(event Collision|EventActorBeginOverlap
  (params (OtherActor :type Actor%20Object%20Reference)))

(event EventTick
  (params (DeltaSeconds :type Float%20%28single-precision%29))
  (bind _output_get (Variables|Default|SettimeAccum (+ DeltaSeconds (Variables|Default|GettimeAccum))))
  (if (>= _output_get (Variables|Default|GettimeMaxForSpawn))
    (Variables|Default|SettimeAccum 0.0)
    (CallFunction|SetNewMaxTimeforSpawn)
    (Game|SpawnActorfromClass "/Game/Blueprints/BP_Vehicle.BP_Vehicle_C" (Transformation|GetActorTransform) "Undefined" 0 (Variables|Default|GetfacingLeft) (Variables|Default|Getspeed) 0 0)))

(fn ConstructionScript)

(fn SetNewMaxTimeforSpawn
  (Variables|Default|SettimeMaxForSpawn (Math|Random|RandomFloatinRange 2.0 5.0)))

(fn SpawnInitialVehicles
  (bind _returnvalue (Transformation|GetActorLocation))
  (bind _returnvalue_2 (Math|Random|RandomFloatinRange 6e+02 1.2e+03))
  (if (Variables|Default|GetfacingLeft)
    (LocalVariables|SetxOffsetInitial (+ (.x _returnvalue) -6e+02))
    (else
      (LocalVariables|SetxOffsetInitial (+ (.x _returnvalue) 6e+02))))
  (while (LocalVariables|GetcontinueCreatingVehicles)
    (LocalVariables|SetxOffsetAccum _returnvalue_2)
    (LocalVariables|SetdistanceAccum (+ _returnvalue_2 (LocalVariables|GetdistanceAccum)))
    (if (Variables|Default|GetfacingLeft)
      (LocalVariables|SetxOffsetAccum (* (LocalVariables|GetxOffsetAccum) -1.0)))
    (Game|SpawnActorfromClass "/Game/Blueprints/BP_Vehicle.BP_Vehicle_C" (Math|Transform|MakeTransform (Math|Vector|MakeVector (+ 0.0 (LocalVariables|GetxOffsetInitial)) (.y _returnvalue) (.z _returnvalue))) "Undefined" 0 (Variables|Default|GetfacingLeft) (Variables|Default|Getspeed) (Variables|Default|GetchickenRef) 0)
    (if (not (>= (LocalVariables|GetdistanceAccum) 6e+03))
      (LocalVariables|SetcontinueCreatingVehicles false))))