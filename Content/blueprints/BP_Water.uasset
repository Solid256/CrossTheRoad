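; Water row floor chunk that spawns three floor sections, landing nodes and optional lily pads or moving logs to cross on.
; Lily pads sit on up to three distinct clear columns and are destroyed with the chunk.
; Logs prefill the row at BeginPlay, then spawn on Tick from one side with random lengths.
; Each log's length sets the gap to the next, and a random per-chunk speed bonus shortens spawn intervals.
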(event EventBeginPlay
  (bind _self self)
  (bind (_transformmid _transformleft _transformright) (CallFunction|CalcFloorTransform))
  (bind _returnvalue (Game|SpawnActorfromClass "/Game/Blueprints/BP_Floor.BP_Floor_C" _transformleft "Undefined" 0 2 false _self 0))
  (Variables|Default|SetleftFloor _returnvalue)
  (bind _returnvalue_2 (Game|SpawnActorfromClass "/Game/Blueprints/BP_Floor.BP_Floor_C" _transformmid "Undefined" 0 2 true _self 0))
  (Variables|Default|SetcenterFloor _returnvalue_2)
  (bind _returnvalue_3 (Game|SpawnActorfromClass "/Game/Blueprints/BP_Floor.BP_Floor_C" _transformright "Undefined" 0 2 false _self 0))
  (Variables|Default|SetrightFloor _returnvalue_3)
  (CallFunction|ConstructLandingNodes)
  (if (Variables|Default|GetcreateLogs)
    (CallFunction|ConstructInitialLogs)))

(event Collision|EventActorBeginOverlap
  (params (OtherActor :type Actor%20Object%20Reference)))

(event EventTick
  (params (DeltaSeconds :type Float%20%28single-precision%29))
  (if (Variables|Default|GetcreateLogs)
    (CallFunction|ConstructLogAttempt DeltaSeconds))
  (CallFunction|CheckifDestroyingFloorChunk))

(event EventDestroyed
  (for _array_element (Variables|Default|GetlillyPads)
    (Actor|DestroyActor _array_element)))

(fn ConstructionScript
  (if (Variables|Default|GetcreateLogs)
    (Variables|Default|SetmaxCreateLogTime (Math|Random|RandomFloatinRange 0.0 1.0))
    (CallFunction|AddExtraLogSpeedRandom)))

(fn ConstructLandingNodes
  (Variables|Default|SetcurZPositionForLandingNode -6e+01)
  (for _index (range 0 8)
    (CallFunction|ConstructLandingNode true))
  (if (Variables|Default|GetcreateLillyPads)
    (CallFunction|ConstructLillyPads)))

(fn ConstructLillyPad
  (params (curX :type Float%20%28single-precision%29))
  (bind _returnvalue (Transformation|GetActorLocation))
  (if (not (== curX -1.0))
    (bind _returnvalue_2 (Game|SpawnActorfromClass "/Game/Blueprints/BP_LillyPad.BP_LillyPad_C" (Math|Transform|MakeTransform (Math|Vector|MakeVector curX (.y _returnvalue) (- (.z _returnvalue) 3e+01))) "Undefined" 0 0))
    (Utilities|Array|Add (Variables|Default|GetlillyPads) _returnvalue_2)))

(fn AddExtraLogSpeedRandom
  (Variables|Default|SetextraLogSpeedCenter (Math|Random|RandomFloatinRange 0.0 2e+02)))

(fn ConstructLogAttempt
  (params (deltaTime :type Float%20%28single-precision%29))
  (bind _extralogspeedcenter (Variables|Default|GetextraLogSpeedCenter))
  (bind _returnvalue (/ _extralogspeedcenter 4e+02))
  (bind _output_get (Variables|Default|SetcurCreateLogTime (+ deltaTime (Variables|Default|GetcurCreateLogTime))))
  (if (>= _output_get (Variables|Default|GetmaxCreateLogTime))
    (if (Variables|Default|GetcreateLogsLeft)
      (CallFunction|ConstructLog -2.8e+03)
      (else
        (CallFunction|ConstructLog 2.8e+03)))
    (Variables|Default|SetcurCreateLogTime 0.0)
    (switch int (Variables|/Game/Blueprints/BP_Log.BP_Log_C|Getlength (Variables|Default|GetcurLogCreated))
      (:1
        (Variables|Default|SetmaxCreateLogTime (- (Math|Random|RandomFloatinRange 1.25 1.5) _returnvalue)))
      (:2
        (Variables|Default|SetmaxCreateLogTime (- (Math|Random|RandomFloatinRange 1.5 1.75) _returnvalue)))
      (:3
        (Variables|Default|SetmaxCreateLogTime (- (Math|Random|RandomFloatinRange 2.0 2.25) _returnvalue))))))

(fn ConstructInitialLogs
  (if (Variables|Default|GetcreateLogsLeft)
    (LocalVariables|SetlogCreatePosX -9e+02)
    (while (< (LocalVariables|GetlogCreatePosX) 9e+02)
      (bind _randomxpos (CallFunction|CalcLogCreationOffsetNext))
      (bind _output_get (LocalVariables|SetlogCreatePosX (+ _randomxpos (LocalVariables|GetlogCreatePosX))))
      (CallFunction|ConstructLog _output_get))
    (else
      (LocalVariables|SetlogCreatePosX 9e+02)
      (while (> (LocalVariables|GetlogCreatePosX) -9e+02)
        (bind _randomxpos_2 (CallFunction|CalcLogCreationOffsetNext))
        (bind _output_get_2 (LocalVariables|SetlogCreatePosX (- (LocalVariables|GetlogCreatePosX) _randomxpos_2)))
        (CallFunction|ConstructLog _output_get_2)))))

(fn ConstructLog
  (params (locationX :type Float%20%28single-precision%29))
  (bind _returnvalue (Transformation|GetActorLocation))
  (bind _returnvalue_2 (Game|SpawnActorfromClass "/Game/Blueprints/BP_Log.BP_Log_C" (Math|Transform|MakeTransform (Math|Vector|MakeVector locationX (.y _returnvalue) (.z _returnvalue))) "Undefined" 0 (Math|Random|RandomIntegerinRange 1 3) (not (Variables|Default|GetcreateLogsLeft)) (Variables|Default|GetextraLogSpeedCenter) 0))
  (bind _output_get (Variables|Default|SetcurLogCreated _returnvalue_2))
  (return _output_get))

(fn ConstructLillyPads
  (bind _numlillypadstocreate (Variables|Default|GetnumLillyPadsToCreate))
  (bind _curclearcolumnposx1 (Variables|Default|GetcurClearColumnPosX1))
  (bind _curclearcolumnposx2 (Variables|Default|GetcurClearColumnPosX2))
  (bind _curclearcolumnposx3 (Variables|Default|GetcurClearColumnPosX3))
  (if (>= _numlillypadstocreate 1)
    (CallFunction|ConstructLillyPad _curclearcolumnposx1)
    (if (>= _numlillypadstocreate 2)
      (if (not (== _curclearcolumnposx1 _curclearcolumnposx2))
        (CallFunction|ConstructLillyPad _curclearcolumnposx2)
        (if (>= _numlillypadstocreate 3)
          (if (not (or (== _curclearcolumnposx2 _curclearcolumnposx3) (== _curclearcolumnposx3 (Variables|Default|GetcurClearColumnPosX1))))
            (CallFunction|ConstructLillyPad _curclearcolumnposx3)))))))

(fn CalcLogCreationOffsetNext
  (bind _curlogcreated (Variables|Default|GetcurLogCreated))
  (Utilities|IsValid _curlogcreated
    (:Is%20Valid
      (switch int (Variables|/Game/Blueprints/BP_Log.BP_Log_C|Getlength _curlogcreated)
        (:1
          (return (Math|Random|RandomFloatinRange 4e+02 5e+02)))
        (:2
          (return (Math|Random|RandomFloatinRange 6e+02 7e+02)))
        (:3
          (return (Math|Random|RandomFloatinRange 8e+02 9e+02)))))
    (:Is%20Not%20Valid
      (return (Math|Random|RandomFloatinRange 0.0 1e+02)))))