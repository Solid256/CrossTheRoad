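; Game mode for a Crossy Road-style chicken game that owns UI, high score, coins, save/reset, restart and a first-person camera toggle.
; Builds the opening grass, then procedurally spawns grass, road, water and railroad chunks up to 20 floors past the player index, scaling chunk sizes with progress.
; Shared clear-column positions place lily pads and shape grass, while water rows limit same-direction log streaks.
; Tick tracks the chicken's furthest row as the score.
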(event EventBeginPlay
  (bind _returnvalue (Game|GetPlayerController 0))
  (Input|EnableInput _returnvalue)
  (Variables|/Script/Engine.PlayerController|SetbShowMouseCursor _returnvalue true)
  (Development|ExecuteConsoleCommand (Variables|Default|GetscreenWindowedCommand) 0)
  (Variables|Default|SetcanRunProgram true)
  (CallFunction|CreateUI)
  (bind _asbp_game_instance (Utilities|Casting|CastToBP_GameInstance (Game|GetGameInstance)))
  (bind _output_get (Variables|Default|SetgameInstanceRef _asbp_game_instance))
  (bind _savegame (Default|AttemptLoadSaveFile _output_get))
  (bind _output_get_2 (Variables|Default|SetsaveGame _savegame))
  (Variables|Default|SethighScore (Variables|/Game/Blueprints/BP_SaveGame.BP_SaveGame_C|GetnumOfFloorsReached _output_get_2))
  (Variables|Default|SetnumOfCoins (Variables|/Game/Blueprints/BP_SaveGame.BP_SaveGame_C|GetnumOfCoins _output_get_2)))

(event EventTick
  (params (DeltaSeconds :type Float%20%28single-precision%29))
  (if (Variables|Default|GetcanRunProgram)
    (if (Variables|Default|GetconstructedInitialChunks)
      (if (Variables|Default|GetstartedGame)
        (Variables|Default|SetstartedGame false)
        (Widget|SetVisibility (Variables|Default|GettitleScreen) "Hidden")
        (Widget|SetVisibility (Variables|Default|GetgameplayUI) "Visible"))
      (CallFunction|CheckChickenChunksExplored)
      (else
        (CallFunction|ConstructInitialFloors)
        (Variables|Default|SetconstructedInitialChunks true)))
    (if (not (Variables|Default|GetgameOver))
      (CallFunction|UpdateHighScore))))

(event Input|ActionEvents|InputActionRestartGame
  (params (Key :type Key%20Structure))
  (bind _savegame (Variables|Default|GetsaveGame))
  (:Pressed
    (if (Variables|Default|GetgameOver)
      (Variables|/Game/Blueprints/BP_SaveGame.BP_SaveGame_C|SetnumOfFloorsReached _savegame (Variables|Default|GethighScore))
      (Variables|/Game/Blueprints/BP_SaveGame.BP_SaveGame_C|SetnumOfCoins _savegame (Variables|Default|GetnumOfCoins))
      (SaveGame|SaveGametoSlot (Variables|Default|GetsaveGame) "save")
      (bind _returnvalue (Game|GetCurrentLevelName true))
      (Audio|PlaySound2D "/Game/Media/Sounds/click.click" 1.0 1.0 0.0 0 0)
      (Game|OpenLevel(byName) (Utilities|String|StringToName _returnvalue)))))

(event Input|ActionEvents|InputActionEraseSaveData
  (params (Key :type Key%20Structure))
  (bind _savegame (Variables|Default|GetsaveGame))
  (:Pressed
    (if (not (Variables|/Game/Blueprints/BP_Chicken.BP_Chicken_C|GethasStarted (Variables|Default|GetchickenRef)))
      (Variables|/Game/Blueprints/BP_SaveGame.BP_SaveGame_C|SetnumOfFloorsReached _savegame 0)
      (Variables|/Game/Blueprints/BP_SaveGame.BP_SaveGame_C|SetnumOfCoins _savegame 0)
      (SaveGame|SaveGametoSlot (Variables|Default|GetsaveGame) "save")
      (Variables|Default|SethighScore 0)
      (Variables|Default|SetnumOfCoins 0)
      (Audio|PlaySound2D "/Game/Media/Sounds/click.click" 1.0 1.0 0.0 0 0))))

(event Input|ActionEvents|InputActionSwitchToFirstPersonMode
  (params (Key :type Key%20Structure))
  (bind _fpcameraref (Variables|Default|GetFPCameraRef))
  (bind _chickenref (Variables|Default|GetchickenRef))
  (bind _chickenref_2 (Variables|Default|GetchickenRef))
  (bind _camera (Variables|/Game/Blueprints/BP_FPCamera.BP_FPCamera_C|GetCamera _fpcameraref))
  (bind _cameraref (Variables|/Game/Blueprints/BP_Chicken.BP_Chicken_C|GetcameraRef _chickenref))
  (bind _staticmesh (Variables|/Game/Blueprints/BP_Chicken.BP_Chicken_C|GetStaticMesh _chickenref_2))
  (bind _camera_2 (Variables|/Game/Blueprints/BP_MainCamera.BP_MainCamera_C|GetCamera _cameraref))
  (:Pressed
    (if (Variables|Default|GetfirstPersonMode)
      (Variables|Default|SetfirstPersonMode false)
      (Components|Activation|SetActive _camera_2 true true)
      (Components|Activation|SetActive _camera false false)
      (Game|Player|SetViewTargetwithBlend (Game|GetPlayerController 0) _cameraref 0.0 "VTBlend_Linear" 0.0 false)
      (if (not (Variables|/Game/Blueprints/BP_Chicken.BP_Chicken_C|GetisDrowned _chickenref_2))
        (Rendering|SetVisibility _staticmesh true false)
        (Audio|Components|Audio|Stop (Variables|Default|GetbackgroundMusic)))
      (else
        (Variables|Default|SetfirstPersonMode true)
        (Components|Activation|SetActive _camera_2 false false)
        (Components|Activation|SetActive _camera true true)
        (Game|Player|SetViewTargetwithBlend (Game|GetPlayerController 0) _fpcameraref 0.0 "VTBlend_Linear" 0.0 false)
        (Rendering|SetVisibility _staticmesh false false)
        (Audio|Components|Audio|Play (Variables|Default|GetbackgroundMusic) 0.0)))))

(event Input|KeyboardEvents|Escape
  (params (Key :type Key%20Structure))
  (:Pressed
    (Game|QuitGame 0 "Quit" false)))

(fn ConstructionScript)

(fn ConstructInitialFloors
  (CallFunction|CreateGrassFloorChunk 8 false)
  (CallFunction|CreateGrassFloorChunk 2 true)
  (CallFunction|ConstructFloors))

(fn CreateGrassFloorChunk
  (params (NumOfFloors :type Integer) (centerClearColumn :type Boolean))
  (if (== (Variables|Default|GetprevFloorTypeCreated) 2)
    _
    (else
      (CallFunction|CreateClearColumnPositions)))
  (if centerClearColumn
    (Variables|Default|SetclearColumnPosX3 0.0))
  (for _index (range 0 (- NumOfFloors 1))
    (Variables|Default|SetcurFloorIndex (+ (Variables|Default|GetcurFloorIndex) 1))
    (bind _posy (CallFunction|CalcFloorSpawnY))
    (Game|SpawnActorfromClass "/Game/Blueprints/BP_Grass.BP_Grass_C" (Math|Transform|MakeTransform (Math|Vector|MakeVector 0.0 _posy 0.0)) "Undefined" 0 (not (== (Math|Integer|%(Integer) _index 2) 0)) (Variables|Default|GetclearColumnPosX1) (Variables|Default|GetclearColumnPosX2) (Variables|Default|GetclearColumnPosX3) _posy (Variables|Default|GetchickenRef) 0)))

(fn CalcFloorSpawnY
  (return (- (* (Variables|Default|GetfloorSpawnYDelta) (Math|Conversions|ToFloat(Integer) (Variables|Default|GetcurFloorIndex))) -2e+02)))

(fn CreateRoadFloorChunk
  (params (NumOfFloors :type Integer))
  (for _index (range 0 (- NumOfFloors 1))
    (Variables|Default|SetcurFloorIndex (+ (Variables|Default|GetcurFloorIndex) 1))
    (bind _posy (CallFunction|CalcFloorSpawnY))
    (Game|SpawnActorfromClass "/Game/Blueprints/BP_Road.BP_Road_C" (Math|Transform|MakeTransform (Math|Vector|MakeVector 0.0 _posy 0.0)) "Undefined" 0 (>= _index 1) _posy (Variables|Default|GetchickenRef) 0)))

(fn CalcCurFloorTypetoCreate
  (Variables|Default|SetprevFloorTypeCreated (Variables|Default|GetcurFloorTypeCreated))
  (Variables|Default|SetcurFloorTypeCreated (Math|Random|RandomInteger 4))
  (if (== (Variables|Default|GetcurFloorTypeCreated) (Variables|Default|GetprevFloorTypeCreated))
    (switch int (Variables|Default|GetprevFloorTypeCreated)
      (:0
        (Variables|Default|SetcurFloorTypeCreated 1))
      (:1
        (Variables|Default|SetcurFloorTypeCreated 2))
      (:2
        (Variables|Default|SetcurFloorTypeCreated 3))
      (:3
        (Variables|Default|SetcurFloorTypeCreated 0)))))

(fn CreateWaterFloorChunk
  (params (NumOfFloors :type Integer))
  (for _index (range 0 (- NumOfFloors 1))
    (Variables|Default|SetcurFloorIndex (+ (Variables|Default|GetcurFloorIndex) 1))
    (bind _posy (CallFunction|CalcFloorSpawnY))
    (if (== (Math|Random|RandomIntegerinRange 0 4) 0)
      (if (Variables|Default|GetcanCreateLillyPads)
        (if (Variables|Default|GetcreatedLillyPadsSinceWaterChunkGroupStarted)
          (CallFunction|CreateClearColumnPositions))
        (CallFunction|CountNumOfLillyPadstoCreate)
        (Game|SpawnActorfromClass "/Game/Blueprints/BP_Water.BP_Water_C" (Math|Transform|MakeTransform (Math|Vector|MakeVector 0.0 _posy 0.0)) "Undefined" 0 false false true (Variables|Default|GetnumOfLillyPadsToCreate) (Variables|Default|GetclearColumnPosX1) (Variables|Default|GetclearColumnPosX2) (Variables|Default|GetclearColumnPosX3) _posy (Variables|Default|GetchickenRef) 0)
        (Variables|Default|SetcreatedLillyPadsSinceWaterChunkGroupStarted true)
        (Variables|Default|SetcanCreateLillyPads false)
        (Variables|Default|SetcreatedLeftLogsSinceLillyPads false)
        (Variables|Default|SetcreatedRightLogsSinceLillyPads false)
        (else
          (bind _output_get (Variables|Default|SetcreateLogsLeft (Math|Random|RandomBool) :!label _label))
          (if (Math|Boolean|Equal(Boolean) _output_get (Variables|Default|GetprevLogCreationDirection))
            (bind _output_get_2 (Variables|Default|SetnumLogsCreatedInSameDirection (+ (Variables|Default|GetnumLogsCreatedInSameDirection) 1)))
            (if (> _output_get_2 2)
              (bind _output_get_3 (Variables|Default|SetcreateLogsLeft (not (Variables|Default|GetcreateLogsLeft))))
              (Variables|Default|SetnumLogsCreatedInSameDirection 1)
              (Variables|Default|SetprevLogCreationDirection _output_get_3))
            (else
              (Variables|Default|SetnumLogsCreatedInSameDirection 1)))
          (Game|SpawnActorfromClass "/Game/Blueprints/BP_Water.BP_Water_C" (Math|Transform|MakeTransform (Math|Vector|MakeVector 0.0 _posy 0.0)) "Undefined" 0 true (Variables|Default|GetcreateLogsLeft) false 0 (Variables|Default|GetclearColumnPosX1) (Variables|Default|GetclearColumnPosX2) (Variables|Default|GetclearColumnPosX3) _posy (Variables|Default|GetchickenRef) 0)
          (if (Variables|Default|GetcreateLogsLeft)
            (Variables|Default|SetcreatedLeftLogsSinceLillyPads true)
            (else
              (Variables|Default|SetcreatedRightLogsSinceLillyPads true)))
          (if (Variables|Default|GetcreatedLeftLogsSinceLillyPads)
            (if (Variables|Default|GetcreatedRightLogsSinceLillyPads)
              (Variables|Default|SetcanCreateLillyPads true)))
          (Variables|Default|SetprevLogCreationDirection (Variables|Default|GetcreateLogsLeft))))
      (else
        (goto _label)))))

(fn CreateRailroadFloorChunk
  (params (NumOfFloors :type Integer))
  (for _index (range 0 (- NumOfFloors 1))
    (Variables|Default|SetcurFloorIndex (+ (Variables|Default|GetcurFloorIndex) 1))
    (bind _posy (CallFunction|CalcFloorSpawnY))
    (Game|SpawnActorfromClass "/Game/Blueprints/BP_Railroad.BP_Railroad_C" (Math|Transform|MakeTransform (Math|Vector|MakeVector 0.0 _posy 0.0)) "Undefined" 0 _posy (Variables|Default|GetchickenRef) 0)))

(fn ConstructFloors
  (bind _numchunksexploredforward (Variables|Default|GetnumChunksExploredForward))
  (bind _numchunksexploredforward_2 (Variables|Default|GetnumChunksExploredForward))
  (bind _returnvalue (/ _numchunksexploredforward 20))
  (bind _returnvalue_2 (/ _numchunksexploredforward_2 20))
  (bind _returnvalue_3 (- 6 _returnvalue))
  (bind _returnvalue_4 (+ 6 _returnvalue_2))
  (bind _returnvalue_5 (Math|Random|RandomInteger _returnvalue_3))
  (bind _returnvalue_6 (Math|Random|RandomInteger _returnvalue_4))
  (bind _returnvalue_7 (+ _returnvalue_6 1))
  (bind _returnvalue_8 (+ _returnvalue_5 1))
  (while (< (- (Variables|Default|GetcurFloorIndex) (Variables|Default|GetplayerPosIndex)) 20)
    (CallFunction|CalcCurFloorTypetoCreate)
    (switch int (Variables|Default|GetcurFloorTypeCreated)
      (:0
        (if (< _returnvalue_8 1)
          (CallFunction|CreateGrassFloorChunk _returnvalue_8 false)
          (else
            (CallFunction|CreateGrassFloorChunk 1 false))))
      (:1
        (CallFunction|CreateRoadFloorChunk _returnvalue_7))
      (:2
        (Variables|Default|SetcreatedLillyPadsSinceWaterChunkGroupStarted false)
        (CallFunction|CreateWaterFloorChunk _returnvalue_7))
      (:3
        (CallFunction|CreateRailroadFloorChunk _returnvalue_7)))))

(fn CreateClearColumnPositions
  (bind _returnvalue (Math|Random|RandomInteger 8))
  (bind _returnvalue_2 (* _returnvalue 2e+02))
  (bind _returnvalue_3 (- _returnvalue_2 8e+02))
  (Variables|Default|SetclearColumnPosX1 -1.0)
  (Variables|Default|SetclearColumnPosX2 -1.0)
  (Variables|Default|SetclearColumnPosX3 -1.0)
  (bind _index (Utilities|FlowControl|ForLoopwithBreak 0 (Math|Random|RandomInteger 2))
    (:LoopBody
      (switch int _index
        (:0
          (Variables|Default|SetclearColumnPosX1 _returnvalue_3))
        (:1
          (Variables|Default|SetclearColumnPosX2 _returnvalue_3))
        (:2
          (Variables|Default|SetclearColumnPosX3 _returnvalue_3))))))

(fn CountNumOfLillyPadstoCreate
  (Variables|Default|SetnumOfLillyPadsToCreate 0)
  (if (!= (Variables|Default|GetclearColumnPosX1) -1.0)
    (Variables|Default|SetnumOfLillyPadsToCreate (+ (Variables|Default|GetnumOfLillyPadsToCreate) 1)))
  (if (!= (Variables|Default|GetclearColumnPosX2) -1.0)
    (Variables|Default|SetnumOfLillyPadsToCreate (+ (Variables|Default|GetnumOfLillyPadsToCreate) 1)))
  (if (!= (Variables|Default|GetclearColumnPosX3) -1.0)
    (Variables|Default|SetnumOfLillyPadsToCreate (+ (Variables|Default|GetnumOfLillyPadsToCreate) 1))))

(fn CheckChickenChunksExplored
  (bind _chickenref (Variables|Default|GetchickenRef))
  (bind _returnvalue (Transformation|GetActorLocation _chickenref))
  (bind _returnvalue_2 (Math|Float|Floor (.y _returnvalue)))
  (bind _returnvalue_3 (Math|Integer|Absolute(Integer) _returnvalue_2))
  (bind _returnvalue_4 (/ _returnvalue_3 200))
  (if (> _returnvalue_4 (Variables|Default|GetnumChunksExploredForward))
    (Variables|Default|SetnumChunksExploredForward _returnvalue_4)))

(fn CreateUI
  (bind _returnvalue (UserInterface|CreateWidget "/Game/UI/BP_TitleScreen.BP_TitleScreen_C" 0 self))
  (bind _output_get (Variables|Default|SettitleScreen _returnvalue))
  (UserInterface|Viewport|AddtoViewport _output_get 0)
  (bind _returnvalue_2 (UserInterface|CreateWidget "/Game/UI/BP_GameplayUI.BP_GameplayUI_C" 0 self))
  (bind _output_get_2 (Variables|Default|SetgameplayUI _returnvalue_2))
  (UserInterface|Viewport|AddtoViewport _output_get_2 0)
  (Widget|SetVisibility _output_get_2 "Hidden"))

(fn UpdateHighScore
  (bind _numchunksexploredforward (Variables|Default|GetnumChunksExploredForward))
  (if (> _numchunksexploredforward (Variables|Default|GethighScore))
    (Variables|Default|SethighScore _numchunksexploredforward)))

(fn PrepPlayerController
  (bind _asbp_player_controller (Utilities|Casting|CastToBP_PlayerController (Game|GetPlayerController 0)))
  (Variables|/Game/Blueprints/BP_PlayerController.BP_PlayerController_C|SetchickenRef _asbp_player_controller (Variables|Default|GetchickenRef)))